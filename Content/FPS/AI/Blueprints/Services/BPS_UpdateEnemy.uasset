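; Behavior tree service that keeps an AI character's blackboard up to date about its current enemy in the FPS game.
; Each tick it clears the enemy through the AI controller if it is invalid or dead.
; Otherwise it checks sight perception for that enemy, sets the on-sight key and toggles the character's aiming to match.
; While the enemy is visible, it also updates a melee-range flag from a fixed distance threshold.
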(event EventReceiveTickAI
  (params (OwnerController :type AI%20Controller%20Object%20Reference) (ControlledPawn :type Pawn%20Object%20Reference) (DeltaSeconds :type Float%20%28single-precision%29))
  (bind _enemykey (Variables|Default|GetEnemyKey))
  (bind _returnvalue (AI|BehaviorTree|GetBlackboardValueasActor _enemykey))
  (bind _asbp_base_character (Utilities|Casting|CastToBP_BaseCharacter _returnvalue))
  (Variables|Default|SetAI_Controller OwnerController)
  (Variables|Default|SetPawn ControlledPawn)
  (Utilities|IsValid _returnvalue
    (:Is%20Valid
      (Variables|Default|SetEnemy _asbp_base_character)
      (if (not (Variables|/Game/FPS/Blueprints/CharacterAndClasses/BP_BaseCharacter.BP_BaseCharacter_C|GetbDead _asbp_base_character))
        (bind _bisonsight (CallFunction|IsEnemyonSight (Variables|Default|GetAI_Controller)))
        (if _bisonsight
          (CallFunction|IsEnemyatMeleeRange)
          (Class|BTFunctionLibrary|SetBlackboardValueasBool (Variables|Default|GetIsOnSightKey) true)
          (bind _asbp_base_ai_character (Utilities|Casting|CastToBP_Base_AI_Character (Variables|Default|GetPawn)))
          (Default|SetAiming _asbp_base_ai_character true)
          (else
            (Class|BTFunctionLibrary|SetBlackboardValueasBool (Variables|Default|GetIsOnSightKey) false)
            (bind _asbp_base_ai_character_2 (Utilities|Casting|CastToBP_Base_AI_Character (Variables|Default|GetPawn)))
            (Default|SetAiming _asbp_base_ai_character_2 false)))
        (else
          (Default|ClearEnemy (.AsBP%20AI%20Player%20Controller (Utilities|Casting|CastToBP_AI_PlayerController (Variables|Default|GetAI_Controller))) :!label _label))))
    (:Is%20Not%20Valid
      (goto _label))))

(fn IsEnemyonSight
  (params (AIController :type AI%20Controller%20Object%20Reference))
  (bind _output_get (LocalVariables|SetEnemy (AI|BehaviorTree|GetBlackboardValueasActor (Variables|Default|GetEnemyKey))))
  (Utilities|IsValid _output_get
    (:Is%20Valid
      (for _array_element (Class|AIPerceptionComponent|GetCurrentlyPerceivedActors (Class|AIController|GetAIPerceptionComponent AIController) "/Script/AIModule.AISense_Sight")
        (if (== _array_element (LocalVariables|GetEnemy))
          (return true))))
    (:Is%20Not%20Valid
      _))
  (return false))

(fn IsEnemyatMeleeRange
  (AI|Components|Blackboard|SetValueasBool (AI|GetBlackboard (Variables|Default|GetAI_Controller)) (Utilities|Name|MakeLiteralName "IsEnemyAtMeleeRange") (< (Math|Vector|VectorLength (- (Transformation|GetActorLocation (Variables|Default|GetPawn)) (Transformation|GetActorLocation (Variables|Default|GetEnemy)))) 1.7e+02)))